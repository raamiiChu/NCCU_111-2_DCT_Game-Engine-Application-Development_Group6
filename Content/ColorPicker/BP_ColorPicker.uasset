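; BP_ColorPicker samples the color under the crosshair and stores it for use as a color picker.
; A looping timer started on BeginPlay reads one pixel from the ColorPicker render target, at the center given by the size variables plus X/Y fine-tune offsets.
; Each read is saved both as a raw color (ColorSTRef) and as a linear color (ColorLRef).
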(event Custom|ColorPicker_event
  ;[1 1 1] 讀取準心上的顏色數值並儲存
  (bind _returnvalue (Class|KismetRenderingLibrary|ReadRenderTargetPixel "/Game/ColorPicker/ColorPicker.ColorPicker" (+ (/ (Variables|Default|GetX_SC_size) 2) (Variables|Default|GetX_FineTune)) (+ (/ (Variables|Default|GetY_SC_size) 2) (Variables|Default|GetY_FineTune))))
  (bind _output_get (Variables|Default|SetcolorST_ref _returnvalue))
  (Variables|Default|SetcolorL_ref (Math|Conversions|ToLinearColor(Color) _returnvalue)))

(event EventBeginPlay
  ;[1 1 1] 讀取準心上的顏色數值並儲存
  (Utilities|Time|SetTimerbyEvent (delegate Custom|ColorPicker_event) 0.1 true))

(fn ConstructionScript)