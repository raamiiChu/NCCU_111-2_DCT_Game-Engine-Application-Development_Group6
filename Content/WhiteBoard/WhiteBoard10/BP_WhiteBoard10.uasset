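; Whiteboard puzzle number 10, where the player draws from a start point to an end point to finish.
; DrawOnWhiteBoard stamps a dynamic marker material onto RT_WhiteBoard10 at the given location and brush size.
; Tick clears the render target whenever the player is not drawing, until the puzzle is finished.
; Start and end checks compare the character's PosX/Y/Z to hardcoded world-space boxes, setting IsFinish when both flags are true.
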(event Custom|Draw%20On%20WhiteBoard
  (params (Location%20To%20Draw :type Vector%202D%20Structure))
  (bind _whiteboardmarker_ml (Variables|Default|GetWhiteBoardMarker_Ml))
  ;[1 1 1] 可改名稱
  (Rendering|Material|SetScalarParameterValue _whiteboardmarker_ml "Draw Size" (Variables|Default|GetdrawSize) :!class /Script/Engine.MaterialInstanceDynamic)
  (Rendering|Material|SetVectorParameterValue _whiteboardmarker_ml "DrawLocation" (Math|Conversions|ToLinearColor(Vector) (Math|Conversions|ToVector(Vector2D) Location%20To%20Draw 0.01)) :!class /Script/Engine.MaterialInstanceDynamic)
  ;[1 1 1] 改 Texture Render Target
  (Rendering|DrawMaterialtoRenderTarget "/Game/WhiteBoard/WhiteBoard10/RT_WhiteBoard10.RT_WhiteBoard10" _whiteboardmarker_ml))

(event Custom|checkIsAtStart
  ;[1 1 1] 檢查是否在起點、終點
  (bind _returnvalue (CallFunction|CheckPosition -2.099e+04 -20979.0 -1.299e+04 -12985.0 1701.0 1712.0))
  (if _returnvalue
    (Variables|Default|SetatStart true)
    (else
      (Variables|Default|SetatStart false))))

(event Custom|checkIsAtEnd
  ;[1 1 1] 檢查是否在起點、終點
  (bind _returnvalue (CallFunction|CheckPosition -21185.0 -21175.0 -12989.0 -12984.0 1754.0 1766.0))
  (if _returnvalue
    (Variables|Default|SetatEnd true)
    ;[1 1 1] 是否通關
    (if (Math|Boolean|ANDBoolean (Variables|Default|GetatStart) (Variables|Default|GetatEnd) (not (Variables|Default|GetisFinish)))
      (Variables|Default|SetisFinish true))
    (else
      (Variables|Default|SetatEnd false))))

(event EventBeginPlay
  (bind _returnvalue (Rendering|Material|CreateDynamicMaterialInstance "/Game/WhiteBoard/M_WhiteBoardMarker.M_WhiteBoardMarker" "None" :!class /Script/Engine.KismetMaterialLibrary))
  (Variables|Default|SetWhiteBoardMarker_Ml _returnvalue)
  ;[1 1 1] 改 Texture Render Target
  (Rendering|ClearRenderTarget2D "/Game/WhiteBoard/WhiteBoard10/RT_WhiteBoard10.RT_WhiteBoard10"))

(event EventTick
  (params (DeltaSeconds :type Float%20%28single-precision%29))
  ;[1 1 1] 獲取是否正在畫圖中，如果尚未通關 & 放開左鍵則畫布清空
  (bind _asfirst_person_character (Utilities|Casting|CastToFirstPersonCharacter (Game|GetPlayerCharacter 0)))
  (if (not (Variables|Default|GetisFinish))
    (if (not (Variables|/Game/FirstPersonBP/Blueprints/FirstPersonCharacter.FirstPersonCharacter_C|Getis%20drawing _asfirst_person_character))
      ;;[1 1 1] 改 Texture Render Target
      (Rendering|ClearRenderTarget2D "/Game/WhiteBoard/WhiteBoard10/RT_WhiteBoard10.RT_WhiteBoard10"))))

(fn ConstructionScript)

(fn CheckPosition
  (params (min_x :type Float%20%28single-precision%29) (max_x :type Float%20%28single-precision%29) (min_y :type Float%20%28single-precision%29) (max_y :type Float%20%28single-precision%29) (min_z :type Float%20%28single-precision%29) (max_z :type Float%20%28single-precision%29))
  (bind _asfirst_person_character (Utilities|Casting|CastToFirstPersonCharacter (Game|GetPlayerCharacter 0)))
  (return (Math|Boolean|ANDBoolean (<= min_x (Variables|/Game/FirstPersonBP/Blueprints/FirstPersonCharacter.FirstPersonCharacter_C|GetposX _asfirst_person_character)) (<= (Variables|/Game/FirstPersonBP/Blueprints/FirstPersonCharacter.FirstPersonCharacter_C|GetposX _asfirst_person_character) max_x) (<= min_y (Variables|/Game/FirstPersonBP/Blueprints/FirstPersonCharacter.FirstPersonCharacter_C|GetposY _asfirst_person_character)) (<= (Variables|/Game/FirstPersonBP/Blueprints/FirstPersonCharacter.FirstPersonCharacter_C|GetposY _asfirst_person_character) max_y) (<= min_z (Variables|/Game/FirstPersonBP/Blueprints/FirstPersonCharacter.FirstPersonCharacter_C|GetposZ _asfirst_person_character)) (<= (Variables|/Game/FirstPersonBP/Blueprints/FirstPersonCharacter.FirstPersonCharacter_C|GetposZ _asfirst_person_character) max_z))))