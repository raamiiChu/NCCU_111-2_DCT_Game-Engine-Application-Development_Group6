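; BP_WhiteBoard12 is a whiteboard drawing puzzle that finishes when start and end checks are both satisfied.
; DrawOnWhiteBoard stamps a dynamic marker material onto RT_WhiteBoard12 at the given location.
; Tick wipes the render target whenever the player stops drawing before completion.
; checkIsAtStart and checkIsAtEnd test the character's PosX/Y/Z against hardcoded boxes, with the end check setting IsFinish.
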(event Custom|Draw%20On%20WhiteBoard
  (params (Location%20To%20Draw :type Vector%202D%20Structure))
  (bind _whiteboardmarker_ml (Variables|Default|GetWhiteBoardMarker_Ml))
  ;[1 1 1] 可改名稱
  (Rendering|Material|SetScalarParameterValue _whiteboardmarker_ml "Draw Size" (Variables|Default|GetdrawSize) :!class /Script/Engine.MaterialInstanceDynamic)
  (Rendering|Material|SetVectorParameterValue _whiteboardmarker_ml "DrawLocation" (Math|Conversions|ToLinearColor(Vector) (Math|Conversions|ToVector(Vector2D) Location%20To%20Draw 0.01)) :!class /Script/Engine.MaterialInstanceDynamic)
  ;[1 1 1] 改 Texture Render Target
  (Rendering|DrawMaterialtoRenderTarget "/Game/WhiteBoard/WhiteBoard12/RT_WhiteBoard12.RT_WhiteBoard12" _whiteboardmarker_ml))

(event Custom|checkIsAtStart
  ;[1 1 1] 檢查是否在起點、終點
  (bind _returnvalue (CallFunction|CheckPosition -14648.0 -14623.0 -9595.0 -9569.0 528.0 535.0))
  (if _returnvalue
    (Variables|Default|SetatStart true)
    (else
      (Variables|Default|SetatStart false))))

(event Custom|checkIsAtEnd
  ;[1 1 1] 檢查是否在起點、終點
  (bind _returnvalue (CallFunction|CheckPosition -14498.0 -14474.0 -9543.0 -9517.0 5.3e+02 5.4e+02))
  (if _returnvalue
    (Variables|Default|SetatEnd true)
    ;[1 1 1] 是否通關
    (if (Math|Boolean|ANDBoolean (Variables|Default|GetatStart) (Variables|Default|GetatEnd) (not (Variables|Default|GetisFinish)))
      (Variables|Default|SetisFinish true))
    (else
      (Variables|Default|SetatEnd false))))

(event EventBeginPlay
  (bind _returnvalue (Rendering|Material|CreateDynamicMaterialInstance "/Game/WhiteBoard/M_WhiteBoardMarker.M_WhiteBoardMarker" "None" :!class /Script/Engine.KismetMaterialLibrary))
  (Variables|Default|SetWhiteBoardMarker_Ml _returnvalue)
  ;[1 1 1] 改 Texture Render Target
  (Rendering|ClearRenderTarget2D "/Game/WhiteBoard/WhiteBoard12/RT_WhiteBoard12.RT_WhiteBoard12"))

(event EventTick
  (params (DeltaSeconds :type Float%20%28single-precision%29))
  ;[1 1 1] 獲取是否正在畫圖中，如果尚未通關 & 放開左鍵則畫布清空
  (bind _asfirst_person_character (Utilities|Casting|CastToFirstPersonCharacter (Game|GetPlayerCharacter 0)))
  (if (not (Variables|Default|GetisFinish))
    (if (not (Variables|/Game/FirstPersonBP/Blueprints/FirstPersonCharacter.FirstPersonCharacter_C|Getis%20drawing _asfirst_person_character))
      ;;[1 1 1] 改 Texture Render Target
      (Rendering|ClearRenderTarget2D "/Game/WhiteBoard/WhiteBoard12/RT_WhiteBoard12.RT_WhiteBoard12"))))

(fn ConstructionScript)

(fn CheckPosition
  (params (miin_x :type Float%20%28single-precision%29) (max_x :type Float%20%28single-precision%29) (miin_y :type Float%20%28single-precision%29) (max_y :type Float%20%28single-precision%29) (miin_z :type Float%20%28single-precision%29) (max_z :type Float%20%28single-precision%29))
  (bind _asfirst_person_character (Utilities|Casting|CastToFirstPersonCharacter (Game|GetPlayerCharacter 0)))
  (return (Math|Boolean|ANDBoolean (<= miin_x (Variables|/Game/FirstPersonBP/Blueprints/FirstPersonCharacter.FirstPersonCharacter_C|GetposX _asfirst_person_character)) (<= (Variables|/Game/FirstPersonBP/Blueprints/FirstPersonCharacter.FirstPersonCharacter_C|GetposX _asfirst_person_character) max_x) (<= miin_y (Variables|/Game/FirstPersonBP/Blueprints/FirstPersonCharacter.FirstPersonCharacter_C|GetposY _asfirst_person_character)) (<= (Variables|/Game/FirstPersonBP/Blueprints/FirstPersonCharacter.FirstPersonCharacter_C|GetposY _asfirst_person_character) max_y) (<= miin_z (Variables|/Game/FirstPersonBP/Blueprints/FirstPersonCharacter.FirstPersonCharacter_C|GetposZ _asfirst_person_character)) (<= (Variables|/Game/FirstPersonBP/Blueprints/FirstPersonCharacter.FirstPersonCharacter_C|GetposZ _asfirst_person_character) max_z))))