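; Whiteboard for a line-drawing puzzle, where a stroke linking a start and an end point completes the board.
; DrawOnWhiteBoard stamps a dynamic marker material into a dedicated render target at the given location and brush size.
; Tick wipes the canvas whenever the first-person player stops drawing before completion.
; Start and end checks copy flags from the first BP_WhiteBoard181 actor and latch IsFinish when both are true.
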(event Custom|Draw%20On%20WhiteBoard
  (params (Location%20To%20Draw :type Vector%202D%20Structure))
  (bind _whiteboardmarker_ml (Variables|Default|GetWhiteBoardMarker_Ml))
  ;[1 1 1] 可改名稱
  (Rendering|Material|SetScalarParameterValue _whiteboardmarker_ml "Draw Size" (Variables|Default|GetdrawSize) :!class /Script/Engine.MaterialInstanceDynamic)
  (Rendering|Material|SetVectorParameterValue _whiteboardmarker_ml "DrawLocation" (Math|Conversions|ToLinearColor(Vector) (Math|Conversions|ToVector(Vector2D) Location%20To%20Draw 0.01)) :!class /Script/Engine.MaterialInstanceDynamic)
  ;[1 1 1] 改 Texture Render Target
  (Rendering|DrawMaterialtoRenderTarget "/Game/WhiteBoard/WhiteBoard18/RT_WhiteBoard18-3.RT_WhiteBoard18-3" _whiteboardmarker_ml))

(event Custom|checkIsAtStart
  ;[1 1 1] 檢查是否在起點、終點
  (bind _outactors (Actor|GetAllActorsOfClass "/Game/WhiteBoard/WhiteBoard18/BP_WhiteBoard18-1.BP_WhiteBoard18-1_C"))
  (if (Variables|/Game/WhiteBoard/WhiteBoard18/BP_WhiteBoard18-1.BP_WhiteBoard18-1_C|GetatStart (Utilities|Array|Get(acopy) _outactors))
    (Variables|Default|SetatStart true)
    (else
      (Variables|Default|SetatStart false))))

(event Custom|checkIsAtEnd
  ;[1 1 1] 檢查是否在起點、終點
  (bind _outactors (Actor|GetAllActorsOfClass "/Game/WhiteBoard/WhiteBoard18/BP_WhiteBoard18-1.BP_WhiteBoard18-1_C"))
  (if (Variables|/Game/WhiteBoard/WhiteBoard18/BP_WhiteBoard18-1.BP_WhiteBoard18-1_C|GetatEnd (Utilities|Array|Get(acopy) _outactors))
    (Variables|Default|SetatEnd true)
    ;[1 1 1] 是否通關
    (if (Math|Boolean|ANDBoolean (Variables|Default|GetatStart) (Variables|Default|GetatEnd) (not (Variables|Default|GetisFinish)))
      (Variables|Default|SetisFinish true))
    (else
      (Variables|Default|SetatEnd false))))

(event EventBeginPlay
  (bind _returnvalue (Rendering|Material|CreateDynamicMaterialInstance "/Game/WhiteBoard/M_WhiteBoardMarker.M_WhiteBoardMarker" "None" :!class /Script/Engine.KismetMaterialLibrary))
  (Variables|Default|SetWhiteBoardMarker_Ml _returnvalue)
  ;[1 1 1] 改 Texture Render Target
  (Rendering|ClearRenderTarget2D "/Game/WhiteBoard/WhiteBoard18/RT_WhiteBoard18-3.RT_WhiteBoard18-3"))

(event EventTick
  (params (DeltaSeconds :type Float%20%28single-precision%29))
  ;[1 1 1] 獲取是否正在畫圖中，如果尚未通關 & 放開左鍵則畫布清空
  (bind _asfirst_person_character (Utilities|Casting|CastToFirstPersonCharacter (Game|GetPlayerCharacter 0)))
  (if (not (Variables|Default|GetisFinish))
    (if (not (Variables|/Game/FirstPersonBP/Blueprints/FirstPersonCharacter.FirstPersonCharacter_C|Getis%20drawing _asfirst_person_character))
      ;;[1 1 1] 改 Texture Render Target
      (Rendering|ClearRenderTarget2D "/Game/WhiteBoard/WhiteBoard18/RT_WhiteBoard18-3.RT_WhiteBoard18-3"))))

(fn ConstructionScript)

(fn CheckPosition
  (params (min_x :type Float%20%28single-precision%29) (maax_x :type Float%20%28single-precision%29) (min_y :type Float%20%28single-precision%29) (maax_y :type Float%20%28single-precision%29) (min_z :type Float%20%28single-precision%29) (maax_z :type Float%20%28single-precision%29))
  (bind _asfirst_person_character (Utilities|Casting|CastToFirstPersonCharacter (Game|GetPlayerCharacter 0)))
  (return (Math|Boolean|ANDBoolean (<= min_x (Variables|/Game/FirstPersonBP/Blueprints/FirstPersonCharacter.FirstPersonCharacter_C|GetposX _asfirst_person_character)) (<= (Variables|/Game/FirstPersonBP/Blueprints/FirstPersonCharacter.FirstPersonCharacter_C|GetposX _asfirst_person_character) maax_x) (<= min_y (Variables|/Game/FirstPersonBP/Blueprints/FirstPersonCharacter.FirstPersonCharacter_C|GetposY _asfirst_person_character)) (<= (Variables|/Game/FirstPersonBP/Blueprints/FirstPersonCharacter.FirstPersonCharacter_C|GetposY _asfirst_person_character) maax_y) (<= min_z (Variables|/Game/FirstPersonBP/Blueprints/FirstPersonCharacter.FirstPersonCharacter_C|GetposZ _asfirst_person_character)) (<= (Variables|/Game/FirstPersonBP/Blueprints/FirstPersonCharacter.FirstPersonCharacter_C|GetposZ _asfirst_person_character) maax_z))))