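; BP_WhiteBoard20-2 is a drawable whiteboard for a trace-style puzzle, paired with BP_WhiteBoard20.
; DrawOnWhiteBoard stamps a dynamic marker material, with size and location parameters, onto its own render target.
; Tick clears that target whenever the first-person character is not drawing, until the board is finished.
; checkFinish sets IsFinish once the first BP_WhiteBoard20 found reports both AtStart and AtEnd.
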(event Custom|Draw%20On%20WhiteBoard
  (params (Location%20To%20Draw :type Vector%202D%20Structure))
  (bind _whiteboardmarker_ml (Variables|Default|GetWhiteBoardMarker_Ml))
  ;[1 1 1] 可改名稱
  (Rendering|Material|SetScalarParameterValue _whiteboardmarker_ml "Draw Size" (Variables|Default|GetdrawSize) :!class /Script/Engine.MaterialInstanceDynamic)
  (Rendering|Material|SetVectorParameterValue _whiteboardmarker_ml "DrawLocation" (Math|Conversions|ToLinearColor(Vector) (Math|Conversions|ToVector(Vector2D) Location%20To%20Draw 0.01)) :!class /Script/Engine.MaterialInstanceDynamic)
  ;[1 1 1] 改 Texture Render Target
  (Rendering|DrawMaterialtoRenderTarget "/Game/WhiteBoard/WhiteBoard20/RT_WhiteBoard20-2.RT_WhiteBoard20-2" _whiteboardmarker_ml))

(event Custom|checkFinish
  ;[1 1 1] 是否通關
  (bind _outactors (Actor|GetAllActorsOfClass "/Game/WhiteBoard/WhiteBoard20/BP_WhiteBoard20.BP_WhiteBoard20_C"))
  (if (Math|Boolean|ANDBoolean (Variables|/Game/WhiteBoard/WhiteBoard20/BP_WhiteBoard20.BP_WhiteBoard20_C|GetatStart (Utilities|Array|Get(acopy) _outactors)) (Variables|/Game/WhiteBoard/WhiteBoard20/BP_WhiteBoard20.BP_WhiteBoard20_C|GetatEnd (Utilities|Array|Get(acopy) _outactors)) (not (Variables|Default|GetisFinish)))
    (Variables|Default|SetisFinish true)))

(event EventBeginPlay
  (bind _returnvalue (Rendering|Material|CreateDynamicMaterialInstance "/Game/WhiteBoard/M_WhiteBoardMarker.M_WhiteBoardMarker" "None" :!class /Script/Engine.KismetMaterialLibrary))
  (Variables|Default|SetWhiteBoardMarker_Ml _returnvalue)
  ;[1 1 1] 改 Texture Render Target
  (Rendering|ClearRenderTarget2D "/Game/WhiteBoard/WhiteBoard20/RT_WhiteBoard20-2.RT_WhiteBoard20-2"))

(event Collision|EventActorBeginOverlap
  (params (OtherActor :type Actor%20Object%20Reference)))

(event EventTick
  (params (DeltaSeconds :type Float%20%28single-precision%29))
  ;[1 1 1] 獲取是否正在畫圖中，如果放開左鍵則畫布清空
  (bind _asfirst_person_character (Utilities|Casting|CastToFirstPersonCharacter (Game|GetPlayerCharacter 0)))
  (if (not (Variables|Default|GetisFinish))
    (if (not (Variables|/Game/FirstPersonBP/Blueprints/FirstPersonCharacter.FirstPersonCharacter_C|Getis%20drawing _asfirst_person_character))
      ;;[1 1 1] 改 Texture Render Target
      (Rendering|ClearRenderTarget2D "/Game/WhiteBoard/WhiteBoard20/RT_WhiteBoard20-2.RT_WhiteBoard20-2"))))

(fn ConstructionScript)