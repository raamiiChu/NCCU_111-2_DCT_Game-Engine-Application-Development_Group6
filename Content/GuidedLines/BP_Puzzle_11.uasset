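; BP_Puzzle_11 is an indicator that lights up when puzzle 11 is solved.
; BeginPlay creates a dynamic M_Emission material on its Cylinder and enables player input, though the graph handles no input events.
; Every Tick it looks up the first BP_WhiteBoard11 and, once both IsFinish and IsFinish2 are true, sets the material's Colour parameter to red.
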(event EventBeginPlay
  (bind _returnvalue (Rendering|Material|CreateDynamicMaterialInstance (Variables|Default|GetCylinder) 0 "/Game/GuidedLines/M_Emission.M_Emission" "None" :!class /Script/Engine.PrimitiveComponent))
  (Input|EnableInput (Game|GetPlayerController 0)))

(event EventTick
  (params (DeltaSeconds :type Float%20%28single-precision%29))
  ;[1 1 1] 過關則亮燈
  ;;[1 1 1] 調取參數，判斷是否過關
  (bind _outactors (Actor|GetAllActorsOfClass "/Game/WhiteBoard/WhiteBoard11/BP_WhiteBoard11.BP_WhiteBoard11_C"))
  (if (and (Variables|/Game/WhiteBoard/WhiteBoard11/BP_WhiteBoard11.BP_WhiteBoard11_C|GetisFinish (Utilities|Array|Get(acopy) _outactors)) (Variables|/Game/WhiteBoard/WhiteBoard11/BP_WhiteBoard11.BP_WhiteBoard11_C|GetisFinish2 (Utilities|Array|Get(acopy) _outactors)))
    (Rendering|Material|SetVectorParameterValue (stale EventBeginPlay _returnvalue) "Colour" "(R=0.683333,G=0.000000,B=0.000000,A=1.000000)" :!class /Script/Engine.MaterialInstanceDynamic)))

(fn ConstructionScript)